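; Custom mission reachpoint actor that stages an example bandit leader encounter during the "Start Up Mission".
; An accepted box overlap caches the mission component, checks the active mission and spawns BP_BanditLeader at a hard-coded transform.
; After a short delay for the sequence change, the leader's AI component follows target locations read from a special objective's follow data.
; Mission targets are then refreshed to account for pawn spawn delay.
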(event OnComponentBeginOverlap(Box)
  (params (OverlappedComponent :type Primitive%20Component%20Object%20Reference) (OtherActor :type Actor%20Object%20Reference) (OtherComp :type Primitive%20Component%20Object%20Reference) (OtherBodyIndex :type Integer) (bFromSweep :type Boolean) (SweepResult :type Hit%20Result%20Structure%20%28by%20ref%29))
  (bind (_canaccess _componentreference) (CallFunction|MissionComponentonOverlap OtherActor))
  (if _canaccess
    (Variables|Default|SetMissionComponent _componentreference)
    ;[0 0 0 1 16] I Know It Should Only Spawn This Actor In This Mission
    (if (CallFunction|IsinSpecificMission? "Start Up Mission")
      ;[0 0 0 1 16] Spawn The Example Bandit Leader
      (bind _returnvalue (Game|SpawnActorfromClass "/Game/MissionComponent/Blueprints/ExampleActors/CustomChilds/BP_BanditLeader.BP_BanditLeader_C" (Math|Transform|MakeTransform "-860.000000,1690.000000,88.000000" "0,-90.000000, 0" "1,1,1") "AlwaysSpawn" 0 0))
      ;[0 0 0 1 16] Wait Untill It Change The Current Sequence
      (Utilities|FlowControl|Delay 0.5)
      ;[0 0 0 1 16] Start NPC To Move
      (Default|MoveNPCtoLocations (Variables|/Game/MissionComponent/Blueprints/ExampleActors/BP_MasterNPC.BP_MasterNPC_C|GetBP_AIComponent _returnvalue) (CallFunction|GetNPCTargets))
      ;[0 0 0 1 16] Refresh The Targets Again, Because We Have To Wait 0.2 Seconds On Pawn Spawn
      (Default|RefreshCurrentTargets (Variables|Default|GetMissionComponent)))))

(event EventBeginPlay
  (|CallParentFunction) ; This node is disabled and will not be called.\nDrag off pins to build functionality.
)

(fn ConstructionScript
  (|CallParentFunction))

(fn GetNPCTargets
  (return (Utilities|Struct|BreakStruct_FollowObjectiveInfo (Utilities|Struct|BreakStruct_SpecialObjectives (Utilities|Struct|BreakStruct_Objectives (Default|FindSpecialObjective (Variables|Default|GetMissionComponent) "NewEnumerator7"))))))
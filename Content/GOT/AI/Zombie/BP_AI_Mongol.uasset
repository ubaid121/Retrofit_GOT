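; Mongol enemy from the Zombie AI folder that plays melee attack animations and is destroyed when struck by a sword.
; EnemyAttack uses a DoOnce gate, a cycling attack counter and delays to pace a three-step combo, though every step currently selects the same montage.
; A Box overlap with an actor tagged "Sword" destroys the enemy instantly; the Box hit event only casts to the base character.
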(event OnComponentHit(Box)
  (params (HitComponent :type Primitive%20Component%20Object%20Reference) (OtherActor :type Actor%20Object%20Reference) (OtherComp :type Primitive%20Component%20Object%20Reference) (NormalImpulse :type Vector :default "0, 0, 0") (Hit :type Hit%20Result%20Structure%20%28by%20ref%29))
  (Utilities|Casting|CastToBP_BaseCharacter_Master (stale OnComponentBeginOverlap(Box) OtherActor)))

(event OnComponentBeginOverlap(Box)
  (params (OverlappedComponent :type Primitive%20Component%20Object%20Reference) (OtherActor :type Actor%20Object%20Reference) (OtherComp :type Primitive%20Component%20Object%20Reference) (OtherBodyIndex :type Integer) (bFromSweep :type Boolean) (SweepResult :type Hit%20Result%20Structure%20%28by%20ref%29))
  (if (Actor|ActorHasTag OtherActor "Sword")
    (Actor|DestroyActor)))

(event EventBeginPlay
  (|CallParentFunction) ; This node is disabled and will not be called.\nDrag off pins to build functionality.
)

(event Collision|EventActorBeginOverlap
  (params (OtherActor :type Actor%20Object%20Reference))
  (|CallParentFunction OtherActor) ; This node is disabled and will not be called.\nDrag off pins to build functionality.
)

(event EventTick
  (params (DeltaSeconds :type Float%20%28single-precision%29))
  (|CallParentFunction DeltaSeconds) ; This node is disabled and will not be called.\nDrag off pins to build functionality.
)

(event EventEnemyAttack
  (Utilities|FlowControl|DoOnce false :!label _label
    (:Completed
      (Animation|Montage|PlayMontage (Variables|Character|GetMesh) (Utilities|Select :Index (Math|Integer|%(Integer) (Variables|Default|GetAttackCount) 3) :Option%200 "/Game/GOT/Animations/Zombie/Zombie_Attack_Montage_01.Zombie_Attack_Montage_01" :Option%201 "/Game/GOT/Animations/Zombie/Zombie_Attack_Montage_01.Zombie_Attack_Montage_01" :Option%202 "/Game/GOT/Animations/Zombie/Zombie_Attack_Montage_01.Zombie_Attack_Montage_01") 1.25
        (:then
          (switch int (Math|Integer|%(Integer) (Variables|Default|GetAttackCount) 3)
            (:Default
              _)
            (:0
              _)
            (:1
              (Math|Integer|IncrementInt (Variables|Default|GetAttackCount)
                (:%20%20
                  (Utilities|FlowControl|Delay 0.8)
                  (Utilities|FlowControl|Sequence
                    (:then_0
                      (goto _label Reset))
                    (:then_1
                      (Utilities|FlowControl|Delay 1.0)
                      (Variables|Default|SetAttackCount 0)
                      (goto _label Reset))))))
            (:2
              (Variables|Default|SetAttackCount 0)
              (Utilities|FlowControl|Delay 1.0)
              (goto _label Reset)))
          (Math|Integer|IncrementInt (Variables|Default|GetAttackCount)
            (:%20%20
              (Utilities|FlowControl|Delay 0.8)
              (Utilities|FlowControl|Sequence
                (:then_0
                  (goto _label Reset))
                (:then_1
                  (Utilities|FlowControl|Delay 0.8)
                  (if (not (> (Variables|Default|GetAttackCount) 1))
                    (Variables|Default|SetAttackCount 0)))))))))))

(fn ConstructionScript
  (|CallParentFunction))
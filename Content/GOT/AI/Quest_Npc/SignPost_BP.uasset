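; SignPost_BP is an interactable signpost that shows its own text in an on-screen dialogue widget.
; The Interactwith event acts as a toggle: it removes and clears the stored widget if one is valid, otherwise it creates a Dialogue_Widget for player controller 0 and adds it to the viewport.
; The new widget's dialogue text is set from the MyText variable.
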(event EventInteractwith
  (Utilities|IsValid (Variables|Default|GetDialgoue_Widget)
    (:Is%20Valid
      (Widget|RemovefromParent (Variables|Default|GetDialgoue_Widget))
      (Variables|Default|SetDialgoue_Widget 0))
    (:Is%20Not%20Valid
      (bind _returnvalue (UserInterface|CreateWidget "/Game/GOT/AI/Quest_Npc/Dialogue_Widget.Dialogue_Widget_C" (Game|GetPlayerController 0)))
      (bind _output_get (Variables|Default|SetDialgoue_Widget _returnvalue))
      (UserInterface|Viewport|AddtoViewport _output_get 0)
      (Variables|/Game/GOT/AI/Quest_Npc/Dialogue_Widget.Dialogue_Widget_C|SetDialougeText (Variables|Default|GetDialgoue_Widget) (Variables|Default|GetMyText)))))

(fn ConstructionScript)
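; Base quest actor that tracks a quest's active and completed subgoals, built from its QuestInfo data.
; Setup activates the starting subgoal indices, with kill counters kept in a parallel array.
; Completing a subgoal activates its listed follow-up subgoals, allowing branching, and directly updates the quest widget's entries and selection.
; A separate function replaces the active set with the subgoal after the highest current index.
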(event EventBeginPlay)

(event Collision|EventActorBeginOverlap
  (params (OtherActor :type Actor%20Object%20Reference)))

(event EventTick
  (params (DeltaSeconds :type Float%20%28single-precision%29)))

(fn ConstructionScript)

(fn UpdateSubgoal
  (Utilities|Array|Clear (Variables|DoNotTouch|GetCurrentGoals))
  (for _array_element (Variables|Donottouch|GetCurrent%20Goal%20Indices)
    (Utilities|Array|Add (Variables|DoNotTouch|GetCurrentGoals) (Utilities|Array|Get(acopy) (.Subgoal (Utilities|Struct|BreakS_Questinfo (Variables|QuestInformation|GetQuestInfo))) _array_element)))
  (return))

(fn SetupStartingGoals
  (Utilities|Array|Clear (Variables|Donottouch|GetCurrent%20Goal%20Indices))
  (Variables|Donottouch|SetCurrent%20Goal%20Indices (Variables|QuestInformation|GetStartingSubgolaIndices))
  (Utilities|Array|Resize (Variables|DoNotTouch|GetCurrent%20Killed%20Amounts) (Utilities|Array|Length (Variables|Donottouch|GetCurrent%20Goal%20Indices)))
  (CallFunction|UpdateSubgoal)
  (Variables|Default|SetCurrent%20Description (.Description (Utilities|Struct|BreakS_Questinfo (Variables|QuestInformation|GetQuestInfo))))
  (return))

(fn Gotonextsubgoal
  (bind _current_goal_indices (Variables|Donottouch|GetCurrent%20Goal%20Indices))
  (bind _current_goal_indices_2 (Variables|Donottouch|GetCurrent%20Goal%20Indices))
  (bind _maxvalue (Math|Integer|MaxOfIntArray _current_goal_indices))
  (bind _returnvalue (+ _maxvalue 1))
  (if (<= _returnvalue (Utilities|Array|LastIndex (.Subgoal (Utilities|Struct|BreakS_Questinfo (Variables|QuestInformation|GetQuestInfo)))))
    (LocalVariables|SetNex%20Index] _returnvalue)
    (Utilities|Array|Clear _current_goal_indices_2)
    (Utilities|Array|Add _current_goal_indices_2 (LocalVariables|GetNex%20Index]))
    (CallFunction|UpdateSubgoal)
    (return true)
    (else
      (return false))))

(fn CompleteSubGoal
  (params (SubGoalIndex :type Integer))
  (bind _questwidget (Variables|DoNotTouch|GetQuestWidget))
  (bind _questwidget_2 (Variables|DoNotTouch|GetQuestWidget))
  (bind _questwidget_3 (Variables|DoNotTouch|GetQuestWidget))
  (bind _current_goal_indices (Variables|Donottouch|GetCurrent%20Goal%20Indices))
  (bind _subgoal_widgets (Variables|/Game/GOT/Quest_info/widget/QuestWidget.QuestWidget_C|GetSubgoal%20Widgets _questwidget))
  (LocalVariables|SetLocal%20Goal%20Index SubGoalIndex)
  (if (Utilities|Array|ContainsItem (Variables|Donottouch|GetCurrent%20Goal%20Indices) (LocalVariables|GetLocal%20Goal%20Index))
    (bind _output_get (LocalVariables|SetLocal%20Completed%20Goal (Utilities|Array|Get(acopy) (.Subgoal (Utilities|Struct|BreakS_Questinfo (Variables|QuestInformation|GetQuestInfo))) (LocalVariables|GetLocal%20Goal%20Index))))
    (Utilities|Array|Add (Variables|DoNotTouch|GetCompletedSubgoals) _output_get)
    (Utilities|Array|RemoveItem (Variables|DoNotTouch|GetCurrentGoals) (LocalVariables|GetLocal%20Completed%20Goal))
    (LocalVariables|SetLocal%20Widget%20Index (Utilities|Array|FindItem _current_goal_indices (LocalVariables|GetLocal%20Goal%20Index)))
    (Utilities|Array|RemoveIndex (Variables|DoNotTouch|GetCurrent%20Killed%20Amounts) (Utilities|Array|FindItem _current_goal_indices (LocalVariables|GetLocal%20Goal%20Index)))
    (Utilities|Array|RemoveItem _current_goal_indices (LocalVariables|GetLocal%20Widget%20Index))
    (Widget|RemovefromParent (Utilities|Array|Get(acopy) _subgoal_widgets (LocalVariables|GetLocal%20Widget%20Index)))
    (Utilities|Array|RemoveIndex _subgoal_widgets (LocalVariables|GetLocal%20Widget%20Index))
    (for _array_element (.FollwingSubGoalIndices (Utilities|Struct|BreakS_GoalInfo (LocalVariables|GetLocal%20Completed%20Goal)))
      (bind _returnvalue (Utilities|Array|Add (Variables|Donottouch|GetCurrent%20Goal%20Indices) _array_element))
      (if (> _returnvalue (Utilities|Array|LastIndex (Variables|DoNotTouch|GetCurrent%20Killed%20Amounts)))
        (Utilities|Array|Add (Variables|DoNotTouch|GetCurrent%20Killed%20Amounts) 0))
      (Utilities|Array|Add (Variables|DoNotTouch|GetCurrentGoals) (Utilities|Array|Get(acopy) (.Subgoal (Utilities|Struct|BreakS_Questinfo (Variables|QuestInformation|GetQuestInfo))) _array_element))
      (bind _returnvalue_2 (UserInterface|CreateWidget "/Game/GOT/Quest_info/widget/SubGoalWidget.SubGoalWidget_C" 0 (Utilities|Array|Get(acopy) (.Subgoal (Utilities|Struct|BreakS_Questinfo (Variables|QuestInformation|GetQuestInfo))) _array_element) self _questwidget_2))
      (Utilities|Array|Add (Variables|/Game/GOT/Quest_info/widget/QuestWidget.QuestWidget_C|GetSubgoal%20Widgets _questwidget_2) _returnvalue_2)
      (Widget|Panel|AddChild (Variables|/Game/GOT/Quest_info/widget/QuestWidget.QuestWidget_C|GetSubGoalBox _questwidget_2) _returnvalue_2))
    (if (== (LocalVariables|GetLocal%20Goal%20Index) (Variables|DoNotTouch|GetSelectedSubgoalindex))
      (Default|SelectSubGoal _questwidget_3 (Utilities|Array|Get(acopy) (Variables|/Game/GOT/Quest_info/widget/QuestWidget.QuestWidget_C|GetSubgoal%20Widgets _questwidget_3))))
    (return true)
    (else
      (return false))))
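; Quest manager actor that spawns and tracks quest actors, handles quest selection and links them to the quest UI.
; AddNewQuest rejects duplicate classes, registers the quest with MainWidget and can auto-select it.
; Kill and object-found events match goal classes across all quests to advance or complete subgoals.
; Subgoal switches spawn a goal marker, with horizontal distance shown on player movement; UpdateDirection and EndQuest are empty stubs.
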(event Custom|On%20switch%20subquest
  (bind _current_quest (Variables|Default|Getcurrent%20quest))
  (bind _mainwidget (Variables|Default|GetMainWidget))
  (Utilities|IsValid (Variables|Default|GetCurrentGoal%20Actor)
    (:Is%20Valid
      (Actor|DestroyActor (Variables|Default|GetCurrentGoal%20Actor)))
    (:Is%20Not%20Valid
      _))
  (bind _output_get (Variables|Default|SetCurrentSubGoal (Utilities|Array|Get(acopy) (.Subgoal (Utilities|Struct|BreakS_Questinfo (Variables|/Game/GOT/Quest_info/Actors/BP_MasterQuests.BP_MasterQuests_C|GetQuestInfo _current_quest))) (Variables|/Game/GOT/Quest_info/Actors/BP_MasterQuests.BP_MasterQuests_C|GetSelectedSubgoalindex _current_quest))))
  (if (.haslocation? (Utilities|Struct|BreakS_Goal_location (.GoalLocation (Utilities|Struct|BreakS_GoalInfo _output_get))))
    (bind _returnvalue (Game|SpawnActorfromClass "/Game/GOT/Quest_info/Actors/BP_goalactor.BP_goalactor_C" (Math|Transform|MakeTransform (.location (Utilities|Struct|BreakS_Goal_location (.GoalLocation (Utilities|Struct|BreakS_GoalInfo _output_get)))) "0, 0, 0" "1,1,1") "AlwaysSpawn" 0 0))
    (Variables|Default|SetCurrentGoal%20Actor _returnvalue)
    (bind _output_get_2 (Variables|Default|SetCurrentDistance (CallFunction|DistancetoGoal)))
    (Rendering|Components|TextRender|SetText (Variables|/Game/GOT/Quest_info/widget/MainWidget_Q.MainWidget_Q_C|GetDistanceText _mainwidget) (Utilities|Text|ToText(Integer) _output_get_2 false false))
    (Widget|SetVisibility _mainwidget (select (> (Variables|Default|GetCurrentDistance) (Variables|Default|GetShow%20Direction%20Amount)) "SelfHitTestInvisible" "Hidden"))
    (else
      (Variables|Default|SetCurrentGoal%20Actor 0)
      (Widget|SetVisibility (Variables|/Game/GOT/Quest_info/widget/MainWidget_Q.MainWidget_Q_C|GetDistanceBorder (Variables|Default|GetMainWidget)) "Hidden"))))

(event Custom|OnPlayMove
  (bind _mainwidget (Variables|Default|GetMainWidget))
  (Utilities|IsValid (Variables|Default|GetCurrentGoal%20Actor)
    (:Is%20Valid
      (bind _output_get (Variables|Default|SetCurrentDistance (CallFunction|DistancetoGoal)))
      (Rendering|Components|TextRender|SetText (Variables|/Game/GOT/Quest_info/widget/MainWidget_Q.MainWidget_Q_C|GetDistanceText _mainwidget) (Utilities|Text|ToText(Integer) _output_get))
      (Math|Integer|CompareInt (Variables|Default|GetCurrentDistance) (Variables|Default|GetShow%20Direction%20Amount)
        (:>
          _)
        (:==
          _)
        (:<
          (Utilities|FlowControl|DoOnce false :!label _label
            (:Completed
              (Widget|SetVisibility _mainwidget "SelfHitTestInvisible")
              (goto _label_2 Reset)))))
      (Utilities|FlowControl|DoOnce false :!label _label_2
        (:Completed
          (Widget|SetVisibility _mainwidget "SelfHitTestInvisible")
          (goto _label Reset))))))

(event Custom|OnEnemyKilled
  (params (Class :type BP%20AI%20Zombie%20Class%20Reference))
  (Variables|Default|SetKilled%20Zombie Class)
  (for (_array_element _array_index) (Variables|Default|GetQuestActors)
    (for (_array_element_2 _array_index_2) (Variables|/Game/GOT/Quest_info/Actors/BP_MasterQuests.BP_MasterQuests_C|GetCurrentGoals _array_element)
      (if (and (Utilities|Enum|Equal(Enum) (.Type (Utilities|Struct|BreakS_GoalInfo _array_element_2)) "NewEnumerator4") (== (.GoalClass (Utilities|Struct|BreakS_GoalInfo _array_element_2)) (Variables|Default|GetKilled%20Zombie)))
        (if (>= (+ (Utilities|Array|Get(acopy) (Variables|/Game/GOT/Quest_info/Actors/BP_MasterQuests.BP_MasterQuests_C|GetCurrent%20Killed%20Amounts _array_element) _array_index) 1) (.Amounttokill (Utilities|Struct|BreakS_GoalInfo _array_element_2)))
          (Default|CompleteSubGoal _array_element (Utilities|Array|Get(acopy) (Variables|/Game/GOT/Quest_info/Actors/BP_MasterQuests.BP_MasterQuests_C|GetCurrent%20Goal%20Indices _array_element) _array_index_2))
          (else
            (Utilities|Array|SetArrayElem (Variables|/Game/GOT/Quest_info/Actors/BP_MasterQuests.BP_MasterQuests_C|GetCurrent%20Killed%20Amounts _array_element) _array_index_2 (+ (Utilities|Array|Get(acopy) (Variables|/Game/GOT/Quest_info/Actors/BP_MasterQuests.BP_MasterQuests_C|GetCurrent%20Killed%20Amounts _array_element) _array_index) 1))
            (Default|Update (Utilities|Array|Get(acopy) (Variables|/Game/GOT/Quest_info/widget/QuestWidget.QuestWidget_C|GetSubgoal%20Widgets (Variables|/Game/GOT/Quest_info/Actors/BP_MasterQuests.BP_MasterQuests_C|GetQuestWidget _array_element)) _array_index_2))))))))

(event Custom|OnObjectFound
  (params (Found%20Object :type Master%20Object%20Class%20Reference))
  (Variables|Default|SetFound%20Object Found%20Object)
  (for _array_element (Variables|Default|GetQuestActors)
    (for (_array_element_2 _array_index) (Variables|/Game/GOT/Quest_info/Actors/BP_MasterQuests.BP_MasterQuests_C|GetCurrentGoals _array_element)
      (if (and (Utilities|Enum|Equal(Enum) (.Type (Utilities|Struct|BreakS_GoalInfo _array_element_2)) "NewEnumerator2") (== (.GoalClass (Utilities|Struct|BreakS_GoalInfo _array_element_2)) (Variables|Default|GetFound%20Object)))
        (Default|CompleteSubGoal _array_element (Utilities|Array|Get(acopy) (Variables|/Game/GOT/Quest_info/Actors/BP_MasterQuests.BP_MasterQuests_C|GetCurrent%20Goal%20Indices _array_element) _array_index))))))

(fn ConstructionScript)

(fn SelectNewQuest
  (params (Quest :type BP%20Master%20Quests%20Object%20Reference) (SubGoal :type Sub%20Goal%20Widgets%20Object%20Reference))
  (Utilities|IsValid (Variables|Default|Getcurrent%20quest)
    (:Is%20Valid
      (Widget|SetIsEnabled (Variables|/Game/GOT/Quest_info/widget/QuestWidget.QuestWidget_C|GetQuestName (Variables|/Game/GOT/Quest_info/Actors/BP_MasterQuests.BP_MasterQuests_C|GetQuestWidget (Variables|Default|Getcurrent%20quest))) false)
      (Default|SelectSubGoal (Variables|/Game/GOT/Quest_info/Actors/BP_MasterQuests.BP_MasterQuests_C|GetQuestWidget (Variables|Default|Getcurrent%20quest))))
    (:Is%20Not%20Valid
      _))
  (bind _output_get (Variables|Default|Setcurrent%20quest Quest))
  (Default|OnQuestSelected (Variables|/Game/GOT/Quest_info/Actors/BP_MasterQuests.BP_MasterQuests_C|GetQuestWidget _output_get))
  (return))

(fn AddNewQuest
  (params (QuestClass :type BP%20Master%20Quests%20Class%20Reference) (DirectlyStart? :type Boolean))
  (bind _mainwidget (Variables|Default|GetMainWidget))
  (LocalVariables|SetLocal%20Class QuestClass)
  (LocalVariables|SetLocal%20Start DirectlyStart?)
  (if (and (Utilities|IsValidClass QuestClass) (not (Utilities|Array|ContainsItem (Variables|Default|GetAllQuestClasses) 0)))
    (Utilities|Array|Add (Variables|Default|GetAllQuestClasses) (LocalVariables|GetLocal%20Class))
    (bind _returnvalue (Game|SpawnActorfromClass (LocalVariables|GetLocal%20Class) (Math|Transform|MakeTransform "0, 0, 0" "0, 0, 0" "1,1,1") "AlwaysSpawn" 0 0))
    (bind _output_get (LocalVariables|SetLocal%20Quest%20Actor _returnvalue))
    (Utilities|Array|Add (Variables|Default|GetQuestActors) _output_get)
    (Default|SetupStartingGoals (LocalVariables|GetLocal%20Quest%20Actor))
    (bind _widget (Default|AddQuesttoList (Variables|Default|GetMainWidget) (LocalVariables|GetLocal%20Quest%20Actor)))
    (bind _output_get_2 (Variables|/Game/GOT/Quest_info/Actors/BP_MasterQuests.BP_MasterQuests_C|SetQuestWidget (LocalVariables|GetLocal%20Quest%20Actor) _widget))
    (Default|UpdateQuest _output_get_2)
    (if (or (LocalVariables|GetLocal%20Start) (<= (Utilities|Array|Length (Variables|Default|GetQuestActors)) 1))
      (CallFunction|SelectNewQuest (LocalVariables|GetLocal%20Quest%20Actor) (Utilities|Array|Get(acopy) (Variables|/Game/GOT/Quest_info/widget/QuestWidget.QuestWidget_C|GetSubgoal%20Widgets (Variables|/Game/GOT/Quest_info/Actors/BP_MasterQuests.BP_MasterQuests_C|GetQuestWidget (LocalVariables|GetLocal%20Quest%20Actor))))))
    (if (Variables|/Game/GOT/Quest_info/widget/MainWidget_Q.MainWidget_Q_C|GetSlideOut? (Variables|Default|GetMainWidget))
      (UserInterface|Animation|PlayAnimation _mainwidget (Variables|/Game/GOT/Quest_info/widget/MainWidget_Q.MainWidget_Q_C|GetSlideOut _mainwidget) 0.0 1 "Reverse" 1.0 false)
      (Variables|/Game/GOT/Quest_info/widget/MainWidget_Q.MainWidget_Q_C|SetSlideOut? _mainwidget false)
      (return true)
      (else
        (return true)))
    (else
      (return false))))

(fn DistancetoGoal
  (bind _third_person_char (Variables|Default|Getthird%20person%20char))
  (bind _currentgoal_actor (Variables|Default|GetCurrentGoal%20Actor))
  (bind _returnvalue (Transformation|GetActorLocation _currentgoal_actor))
  (bind _returnvalue_2 (Transformation|GetActorLocation _third_person_char))
  (return (Math|Float|Round (/ (Math|Vector|VectorLength (- (Math|Vector|MakeVector (.x _returnvalue_2) (.y _returnvalue_2) 0.0) (Math|Vector|MakeVector (.x _returnvalue) (.y _returnvalue) 0.0))) 1e+02))))

(fn UpdateDirection)

(fn EndQuest
  (params (Quest :type BP%20Master%20Quests%20Object%20Reference)))
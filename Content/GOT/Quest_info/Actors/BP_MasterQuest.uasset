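; BP_MasterQuest is a quest actor, apparently a base for individual quests, that tracks which subgoals from its QuestInfo are current.
; SetupStartingGoals loads the starting indices, and UpdateSubgoal rebuilds the current goal list from the active indices.
; Gotonextsubgoal replaces all active indices with the one after the highest, returning false when none remains.
; It has no active event logic, so these functions rely on outside callers.
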(event EventBeginPlay)

(event Collision|EventActorBeginOverlap
  (params (OtherActor :type Actor%20Object%20Reference)))

(event EventTick
  (params (DeltaSeconds :type Float%20%28single-precision%29)))

(fn ConstructionScript)

(fn UpdateSubgoal
  (Utilities|Array|Clear (Variables|DoNotTouch|GetCurrentGOals))
  (for _array_element (Variables|Donottouch|GetCurrentgoalIndices)
    (Utilities|Array|Add (Variables|DoNotTouch|GetCurrentGOals) (Utilities|Array|Get(acopy) (.Subgoal (Utilities|Struct|BreakS_Questinfo (Variables|QuestInformation|GetQuestInfo))) _array_element)))
  (return))

(fn SetupStartingGoals
  (Utilities|Array|Clear (Variables|Donottouch|GetCurrentgoalIndices))
  (Variables|Donottouch|SetCurrentgoalIndices (Variables|QuestInformation|GetStartingSubgolaIndices))
  (CallFunction|UpdateSubgoal)
  (return))

(fn Gotonextsubgoal
  (bind _currentgoalindices (Variables|Donottouch|GetCurrentgoalIndices))
  (bind _currentgoalindices_2 (Variables|Donottouch|GetCurrentgoalIndices))
  (bind _maxvalue (Math|Integer|MaxOfIntArray _currentgoalindices))
  (bind _returnvalue (+ _maxvalue 1))
  (if (<= _returnvalue (Utilities|Array|LastIndex (.Subgoal (Utilities|Struct|BreakS_Questinfo (Variables|QuestInformation|GetQuestInfo)))))
    (LocalVariables|SetNex%20Index] _returnvalue)
    (Utilities|Array|Clear _currentgoalindices_2)
    (Utilities|Array|Add _currentgoalindices_2 (LocalVariables|GetNex%20Index]))
    (CallFunction|UpdateSubgoal)
    (return true)
    (else
      (return false))))